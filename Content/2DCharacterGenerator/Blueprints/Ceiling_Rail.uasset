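; Ceiling rail actor for a 2D game, built from a Rope box and two end blocks, with an adjustable length.
; The construction script sizes the box along X from BoxXExtent, then moves BlockLeft and BlockRight just beyond and below its ends.
; The event graph holds only disabled stub events, so the actor has no runtime logic of its own.
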(event `self.ReceiveBeginPlay`)

(event `self.ReceiveActorBeginOverlap`
  (params (OtherActor :type "Actor Object Reference")))

(event `self.ReceiveTick`
  (params (DeltaSeconds :type "Float (single-precision)")))

(fn `UserConstructionScript`
  (bind _returnvalue (+ (.x (`BoxComponent.BoxExtent` (`self.Rope`))) 35.0))
  ;[0.564 1 0.612] Set Box Extent
  (`BoxComponent.SetBoxExtent` (`self.Rope`) (`KismetMathLibrary.MakeVector` (`self.Box X Extent`) 1.0 5.0) true)
  (`SceneComponent.K2_SetRelativeLocation` (`self.BlockLeft`) (`KismetMathLibrary.MakeVector` (* _returnvalue -1.0) 0.0 -32.0) false)
  (`SceneComponent.K2_SetRelativeLocation` (`self.BlockRight`) (`KismetMathLibrary.MakeVector` _returnvalue 0.0 -32.0) false))