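; Level-design tool actor that builds a 2D platform or wall from Paper2D sprites in its construction script.
; It pins itself to Y=0 and tiles a configurable number of middle sprites along X, spaced by sprite bounds.
; Optional rotatable edge sprites cap both ends, the right one yawed 180 degrees.
; All pieces are WorldStatic, tagged floor or wall; a DestroyComponent event removes a given sprite when Destructible.
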(event `self.ReceiveBeginPlay`)

(event `self.ReceiveActorBeginOverlap`
  (params (OtherActor :type "Actor Object Reference")))

(event `self.ReceiveTick`
  (params (DeltaSeconds :type "Float (single-precision)")))

(event `Destroy Component`
  (params (`Sprite Component` :type "PrimitiveComponent Object Reference"))
  (if (`self.Destructible`)
    (`ActorComponent.K2_DestroyComponent` `Sprite Component`)))

(fn `UserConstructionScript`
  (bind _spritecenterarray (`self.SpriteCenterArray`))
  (bind _scale (`self.Scale`))
  (bind _scale_2 (`self.Scale`))
  (bind _scale_3 (`self.Scale`))
  (bind _returnvalue (* (.x (`.BoxExtent` (`KismetSystemLibrary.GetComponentBounds` (`KismetArrayLibrary.Array_Get` (`self.SpriteCenterArray`))))) 2.0))
  (`self.K2_SetActorLocation` (`KismetMathLibrary.MakeVector` (.x (`self.K2_GetActorLocation`)) 0.0 (.z (`self.K2_GetActorLocation`))))
  (set `self.NumberOfspriteInMidle` (`KismetMathLibrary.Max` (`self.NumberOfspriteInMidle`) 1))
  (for _index (range 1 (+ (`self.NumberOfspriteInMidle`) 1))
    (bind _returnvalue_2 (`AddComponent|Paper Sprite Component_254` :`RelativeTransform` (`KismetMathLibrary.MakeTransform` (`KismetMathLibrary.MakeVector` (- (* (`KismetMathLibrary.Conv_IntToDouble` _index) _returnvalue) _returnvalue)) (struct) (`KismetMathLibrary.MakeVector` _scale _scale _scale))))
    (`KismetArrayLibrary.Array_AddUnique` (`self.SpriteCenterArray`) _returnvalue_2)
    (`PaperSpriteComponent.SetSprite` _returnvalue_2 (`self.SpriteCenter`))
    (`PrimitiveComponent.SetCollisionObjectType` _returnvalue_2 "ECC_WorldStatic")
    (if (`self.FloorTrueWallFalse`)
      (set `ActorComponent.ComponentTags` (`|MakeArray` "floor" :!type "Name") _returnvalue_2)
      (else
        (set `ActorComponent.ComponentTags` (`|MakeArray` "wall" :!type "Name") _returnvalue_2))))
  (if (`self.Edges`)
    (`|ExecutionSequence`
      (:`then_0`
        (bind _returnvalue_3 (`AddComponent|PaperSpriteComponent_5713` :`RelativeTransform` (`KismetMathLibrary.MakeTransform` (`KismetMathLibrary.MakeVector` (- (.x (`SceneComponent.RelativeLocation` (`KismetArrayLibrary.Array_Get` (`self.SpriteCenterArray`)))) (* (.x (`.BoxExtent` (`KismetSystemLibrary.GetComponentBounds` (`KismetArrayLibrary.Array_Get` (`self.SpriteCenterArray`))))) 2.0))) (`KismetMathLibrary.MakeRot` (`self.LeftEdgeRotation`) 0.0) (`KismetMathLibrary.MakeVector` _scale_2 _scale_2 _scale_2))))
        (`PaperSpriteComponent.SetSprite` _returnvalue_3 (`self.SpriteEdgeLeft`))
        (set `self.Bounds` (`.BoxExtent` (`KismetSystemLibrary.GetComponentBounds` _returnvalue_3)))
        (`PrimitiveComponent.SetCollisionObjectType` _returnvalue_3 "ECC_WorldStatic")
        (if (`self.FloorTrueWallFalse`)
          (set `ActorComponent.ComponentTags` (`|MakeArray` "floor" :!type "Name") _returnvalue_3)
          (else
            (set `ActorComponent.ComponentTags` (`|MakeArray` "wall" :!type "Name") _returnvalue_3))))
      (:`then_1`
        (bind _returnvalue_4 (`AddComponent|PaperSpriteComponent_5714` :`RelativeTransform` (`KismetMathLibrary.MakeTransform` (`KismetMathLibrary.MakeVector` (+ (.x (`SceneComponent.RelativeLocation` (`KismetArrayLibrary.Array_Get` _spritecenterarray (`KismetArrayLibrary.Array_LastIndex` _spritecenterarray)))) (* (.x (`.BoxExtent` (`KismetSystemLibrary.GetComponentBounds` (`KismetArrayLibrary.Array_Get` (`self.SpriteCenterArray`))))) 2.0))) (`KismetMathLibrary.MakeRot` (`self.RightEdgeRotation`) 180.0) (`KismetMathLibrary.MakeVector` _scale_3 _scale_3 _scale_3))))
        (`PaperSpriteComponent.SetSprite` _returnvalue_4 (`self.SpriteEdgeRight`))
        (set `self.Bounds` (`.BoxExtent` (`KismetSystemLibrary.GetComponentBounds` _returnvalue_4)))
        (`PrimitiveComponent.SetCollisionObjectType` _returnvalue_4 "ECC_WorldStatic")
        (if (`self.FloorTrueWallFalse`)
          (set `ActorComponent.ComponentTags` (`|MakeArray` "floor" :!type "Name") _returnvalue_4)
          (else
            (set `ActorComponent.ComponentTags` (`|MakeArray` "wall" :!type "Name") _returnvalue_4)))))))