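; Default 2D projectile actor that displays a tinted sprite and reacts to hitting level geometry.
; On begin play it applies a dynamic instance of the BlockOut material to the sprite, setting partial desaturation and the projectile's Color.
; When the sprite overlaps a component tagged floor or wall, it spawns HitClass at the Impact component's location and destroys itself.
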(event `self.ReceiveBeginPlay`
  (bind _material_inst (`self.Material Inst`))
  ;[0.5317 1 0.4761] Begin Play Set Dynamic Material
  (bind _returnvalue (`PrimitiveComponent.CreateDynamicMaterialInstance` 0 "/Game/2DCharacterGenerator/Material/BlockOut_Inst.BlockOut_Inst"))
  (bind _output_get (set `self.Material Inst` _returnvalue))
  (`PrimitiveComponent.SetMaterial` (`self.Projectile Sprite`) 0 _output_get)
  (`MaterialInstanceDynamic.SetScalarParameterValue` _material_inst "Desaturation" 0.7)
  (`MaterialInstanceDynamic.SetVectorParameterValue` _material_inst "Color" (`self.Color`)))

(event `self.Projectile Sprite.OnComponentBeginOverlap`
  (params (OtherActor :type "Actor Object Reference") (OtherComp :type "PrimitiveComponent Object Reference") (OtherBodyIndex :type Integer) (bFromSweep :type Boolean) (SweepResult :type "EngineTypes.HitResult Structure (by ref)"))
  ;[1 0.1638 0.14] Projectile Hit
  (if (or (`ActorComponent.ComponentHasTag` OtherComp "floor") (`ActorComponent.ComponentHasTag` OtherComp "wall"))
    (`|SpawnActorFromClass` (`self.Hit class`) (`KismetMathLibrary.MakeTransform` (`SceneComponent.K2_GetComponentLocation` (`self.Impact`))))
    (`self.K2_DestroyActor` self)))

(fn `UserConstructionScript`)